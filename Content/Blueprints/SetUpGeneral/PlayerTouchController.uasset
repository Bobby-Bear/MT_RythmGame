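; Player controller that tracks mouse and touch drags as world-space start and current positions on the X and Z axes.
; On press, it stores the Visibility trace hit under the cursor or first finger as the start location and opens that input's gate.
; While a gate is open, Tick (and touch movement) re-traces to update the current location until release.
; MoveToHitLocation only stores coordinates; it moves nothing itself.
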(event `self.ReceiveTick`
  (params (DeltaSeconds :type "Float (single-precision)"))
  (`|ExecutionSequence`
    (:`then_0`
      (`/Engine/EditorBlueprintResources/StandardMacros.Gate` true :!label _label
        (:`Exit`
          (`self.Move to Hit Location` (`self.GetHitResultUnderCursorByChannel` "TraceTypeQuery1")))))
    (:`then_1`
      (`/Engine/EditorBlueprintResources/StandardMacros.Gate` true :!label _label_2
        (:`Exit`
          (`self.Move to Hit Location` (`self.GetHitResultUnderFingerByChannel` "Touch1" "TraceTypeQuery1")))))))

(event `InputAction|MouseTouch`
  (params (Key :type "Key Structure"))
  (bind _hitresult (`self.GetHitResultUnderCursorByChannel` "TraceTypeQuery1"))
  (:`Pressed`
    (set `self.Start LocationX` (.x (`.Location` (`GameplayStatics.BreakHitResult` _hitresult))))
    (set `self.Start LocationZ` (.z (`.Location` (`GameplayStatics.BreakHitResult` _hitresult))))
    (goto _label :!via `Open`))
  (:`Released`
    (goto _label :!via `Close`)))

(event `InputTouch`
  (params (Location :type "Vector Structure") (FingerIndex :type "ETouchIndex Enum"))
  (bind _hitresult (`self.GetHitResultUnderFingerByChannel` "Touch1" "TraceTypeQuery1"))
  (:`Pressed`
    (set `self.Start LocationX` (.x (`.Location` (`GameplayStatics.BreakHitResult` _hitresult))))
    (set `self.Start LocationZ` (.z (`.Location` (`GameplayStatics.BreakHitResult` _hitresult))))
    (goto _label_2 :!via `Open`))
  (:`Released`
    (goto _label_2 :!via `Close`))
  (:`Moved`
    (goto _label_2)))

(fn `Move to Hit Location`
  (params (NewParam :type "HitResult Structure"))
  (bind (_bblockinghit _binitialoverlap _time _distance _location) (`GameplayStatics.BreakHitResult` NewParam))
  (set `self.Current LocationX` (.x _location))
  (set `self.Current LocationZ` (.z _location)))

(fn `UserConstructionScript`)