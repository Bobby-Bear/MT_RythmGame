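; SpinCircle is a touch-driven sprite actor that rotates in pitch and destroys itself on a short timer after BeginPlay.
; Sprite touches open a gate, fed by Tick and touch events, that traces under the finger; releasing closes it.
; Start and current X/Z are both sampled on each pass, and their Atan2 difference, with swapped arguments, is added to the rotation only when at least the current rotation.
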(event `SetTimer`
  (`KismetSystemLibrary.K2_SetTimerDelegate` (delegate `SelfDestruct`) 5.0))

(event `self.ReceiveBeginPlay`
  (`self.SetTimer`))

(event `SelfDestruct`
  (`self.K2_DestroyActor`))

(event `self.ReceiveTick`
  (params (DeltaSeconds :type "Float (single-precision)"))
  (bind _returnvalue (`GameplayStatics.GetPlayerController` 0))
  (bind _current_rotation (`self.Current Rotation`))
  (bind _returnvalue_2 (- (`KismetMathLibrary.DegAtan2` (`self.LocationCurrentX`) (`self.LocationCurrentZ`)) (`KismetMathLibrary.DegAtan2` (`self.LocationStartZ`) (`self.LocationStartX`))))
  (`/Engine/EditorBlueprintResources/StandardMacros.Gate` true :!label _label
    (:`Exit`
      (bind (_bblockinghit _binitialoverlap _time _distance _location) (`GameplayStatics.BreakHitResult` (`PlayerController.GetHitResultUnderFingerByChannel` _returnvalue (stale `self.PaperSprite.OnInputTouchBegin` FingerIndex) "TraceTypeQuery1" true)))
      (set `self.LocationStartX` (.x _location))
      (set `self.LocationStartZ` (.z _location))
      (bind (_bblockinghit_2 _binitialoverlap_2 _time_2 _distance_2 _location_2) (`GameplayStatics.BreakHitResult` (`PlayerController.GetHitResultUnderFingerByChannel` _returnvalue (stale `InputTouch` FingerIndex) "TraceTypeQuery1" true)))
      (set `self.LocationCurrentX` (.x _location_2))
      (set `self.LocationCurrentZ` (.z _location_2))
      (if (>= _returnvalue_2 _current_rotation)
        (set `self.Current Rotation` (+ _current_rotation _returnvalue_2)))
      (`self.K2_SetActorRotation` (`KismetMathLibrary.MakeRotator` 0.0 (`self.Current Rotation`))))))

(event `self.PaperSprite.OnInputTouchBegin`
  (params (FingerIndex :type "ETouchIndex Enum" :default "Touch1") (TouchedComponent :type "PrimitiveComponent Object Reference"))
  (goto _label :!via `Open`))

(event `InputTouch`
  (params (Location :type "Vector Structure") (FingerIndex :type "ETouchIndex Enum"))
  (:`Pressed`
    (goto _label))
  (:`Released`
    (goto _label :!via `Close`))
  (:`Moved`
    (goto _label)))

(event `self.PaperSprite.OnInputTouchEnd`
  (params (FingerIndex :type "ETouchIndex Enum" :default "Touch1") (TouchedComponent :type "PrimitiveComponent Object Reference"))
  (goto _label :!via `Close`))

(fn `UserConstructionScript`)