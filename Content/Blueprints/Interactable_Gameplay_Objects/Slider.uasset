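; Timed slider gameplay object that shows a shrinking approach sprite, then slides a cube from Point1 to Point2 and destroys itself.
; Tick scales PaperSprite1 down over ReactionTime, calling SlideSquare once it is small enough to start the SliderDuration timer.
; Timer elapsed time drives both phases, with the cube's X/Z position interpolated by hand in branches on the points' relative positions and moved with sweep.
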(event `self.ReceiveTick`
  (params (DeltaSeconds :type "Float (single-precision)"))
  (bind _scalez (`self.ScaleZ`))
  (bind _reaction_time (`self.Reaction Time`))
  (bind _scalex (`self.ScaleX`))
  (bind (_returnvalue_x _returnvalue_y _returnvalue_z) (`KismetMathLibrary.BreakVector` (`SceneComponent.K2_GetComponentLocation` (`self.Point1`))))
  (bind (_returnvalue_x_2 _returnvalue_y_2 _returnvalue_z_2) (`KismetMathLibrary.BreakVector` (`SceneComponent.K2_GetComponentLocation` (`self.Point1`))))
  (bind (_returnvalue_x_3 _returnvalue_y_3 _returnvalue_z_3) (`KismetMathLibrary.BreakVector` (`SceneComponent.K2_GetComponentLocation` (`self.Point1`))))
  (bind (_returnvalue_x_4 _returnvalue_y_4 _returnvalue_z_4) (`KismetMathLibrary.BreakVector` (`SceneComponent.K2_GetComponentLocation` (`self.Point1`))))
  (bind (_returnvalue_x_5 _returnvalue_y_5 _returnvalue_z_5) (`KismetMathLibrary.BreakVector` (`SceneComponent.K2_GetComponentLocation` (`self.Point1`))))
  (bind (_returnvalue_x_6 _returnvalue_y_6 _returnvalue_z_6) (`KismetMathLibrary.BreakVector` (`SceneComponent.K2_GetComponentLocation` (`self.Point2`))))
  (`/Engine/EditorBlueprintResources/StandardMacros.Gate` true :!label _label
    (:`Exit`
      (if (not (`self.SquareShrinkComplete`))
        (set `self.Reaction Time` _reaction_time)
        (bind _returnvalue (* (/ (- _reaction_time (`KismetSystemLibrary.K2_GetTimerElapsedTimeHandle` (stale `Start Timer` _returnvalue))) (`self.Reaction Time`)) (`self.DefaultScale`)))
        (set `self.ScaleX` _returnvalue)
        (set `self.ScaleZ` _returnvalue)
        (`SceneComponent.SetWorldScale3D` (`self.PaperSprite1`) (`KismetMathLibrary.MakeVector` _scalex 0.0 _scalez))
        (if (and (< _scalex 0.5) (< _scalez 0.5))
          (`self.Slide Square`))
        (elif (and (<= _returnvalue_x_5 _returnvalue_x_6) (<= _returnvalue_z_5 _returnvalue_z_6))
          (bind _returnvalue_2 (* (/ (`KismetSystemLibrary.K2_GetTimerElapsedTimeHandle` (stale `Slide Square` _returnvalue)) (`self.Slider Duration`)) -1.0))
          (bind _returnvalue_3 (* (- _returnvalue_x_5 _returnvalue_x_6) _returnvalue_2))
          (bind _returnvalue_4 (* _returnvalue_2 (- _returnvalue_z_5 _returnvalue_z_6)))
          (`SceneComponent.K2_SetWorldLocation` (`self.Cube`) (`KismetMathLibrary.MakeVector` (+ _returnvalue_3 _returnvalue_x) 0.0 (+ _returnvalue_z _returnvalue_4)) true false)
          (elif (and (> _returnvalue_x_5 _returnvalue_x_6) (< _returnvalue_z_5 _returnvalue_z_6))
            (`SceneComponent.K2_SetWorldLocation` (`self.Cube`) (`KismetMathLibrary.MakeVector` (- _returnvalue_3 _returnvalue_x_2) 0.0 (+ _returnvalue_z_2 _returnvalue_4)) true false)
            (elif (and (>= _returnvalue_x_5 _returnvalue_x_6) (>= _returnvalue_z_5 _returnvalue_z_6))
              (`SceneComponent.K2_SetWorldLocation` (`self.Cube`) (`KismetMathLibrary.MakeVector` (+ _returnvalue_3 _returnvalue_x_3) 0.0 (+ _returnvalue_z_3 _returnvalue_4)) true false)
              (else
                (`SceneComponent.K2_SetWorldLocation` (`self.Cube`) (`KismetMathLibrary.MakeVector` (+ _returnvalue_3 _returnvalue_x_4) 0.0 (+ _returnvalue_z_4 _returnvalue_4)) true false)))))))))

(event `self.ReceiveBeginPlay`
  (`self.Start Timer`)
  (goto _label :!via `Open`))

(event `Start Timer`
  (bind _returnvalue (`KismetSystemLibrary.K2_SetTimerDelegate` (delegate `Dummy`) (`self.Reaction Time`))))

(event `Dummy`)

(event `Slide Square`
  (set `self.SquareShrinkComplete` true)
  (bind _returnvalue (`KismetSystemLibrary.K2_SetTimerDelegate` (delegate `Destroy Slider`) (`self.Slider Duration`))))

(event `Destroy Slider`
  (`self.K2_DestroyActor`))

(fn `UserConstructionScript`)

(fn `WhichQuadrant`)