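; Square is a timed gameplay actor whose sprite shrinks over its ReactionTime before the actor destroys itself.
; BeginPlay starts a one-shot timer that calls DestroySquare and opens a gate on Tick.
; Each tick scales the sprite's X and Z from DefaultScale by the fraction of time remaining, forming a visual countdown.
; The Cube's touch event is present but has no logic.
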(event `self.ReceiveTick`
  (params (DeltaSeconds :type "Float (single-precision)"))
  (`/Engine/EditorBlueprintResources/StandardMacros.Gate` true :!label _label
    (:`Exit`
      (bind _returnvalue (* (/ (- (`self.Reaction Time`) (`KismetSystemLibrary.K2_GetTimerElapsedTimeHandle` (stale `Start Timer` _returnvalue))) (`self.Reaction Time`)) (`self.DefaultScale`)))
      (set `self.ScaleX` _returnvalue)
      (set `self.ScaleZ` _returnvalue)
      (`SceneComponent.SetWorldScale3D` (`self.PaperSprite`) (`KismetMathLibrary.MakeVector` (`self.ScaleX`) 0.0 (`self.ScaleZ`))))))

(event `self.ReceiveBeginPlay`
  (`self.Start Timer`)
  (goto _label :!via `Open`))

(event `self.Cube.OnInputTouchBegin`
  (params (FingerIndex :type "ETouchIndex Enum" :default "Touch1") (TouchedComponent :type "PrimitiveComponent Object Reference")))

(event `Start Timer`
  (bind _returnvalue (`KismetSystemLibrary.K2_SetTimerDelegate` (delegate `DestroySquare`) (`self.Reaction Time`))))

(event `DestroySquare`
  (`self.K2_DestroyActor`))

(fn `UserConstructionScript`)